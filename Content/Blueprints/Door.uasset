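; A maze door that the player opens by spending a Skull Key of its key type, with its material looked up from the game instance.
; Overlapping the trigger volume enables Interact input and shows a HUD prompt through the game mode.
; Interacting decrements the player's key count, updates the HUD and attaches a matching key mesh to the keyhole.
; A timeline then moves key and door with sound, and destroys the actor when finished.
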(event `self.ReceiveBeginPlay`
  (bind _asmaze_game_instance (cast `/Game/GameMode/MazeGameInstance` (`GameplayStatics.GetGameInstance`)))
  (`PrimitiveComponent.SetMaterial` (`self.DoorMesh`) 1 (`BlueprintMapLibrary.Map_Find` (`/Game/GameMode/MazeGameInstance.KeyTypes` _asmaze_game_instance) (`self.KeyTypeEnum`))))

(event `self.TriggerVolume.OnComponentBeginOverlap`
  (params (OverlappedComponent :type "PrimitiveComponent Object Reference") (OtherActor :type "Actor Object Reference") (OtherComp :type "PrimitiveComponent Object Reference") (OtherBodyIndex :type Integer) (bFromSweep :type Boolean) (SweepResult :type "HitResult Structure (by ref)"))
  (bind _returnvalue (`GameplayStatics.GetPlayerCharacter` 0))
  (if (`self.open`)
    _
    (elif (== OtherActor _returnvalue)
      (`self.EnableInput` (`GameplayStatics.GetPlayerController` 0))
      (bind _asplayer_character (cast `/Game/Player/PlayerCharacter` _returnvalue))
      (if (> (`BlueprintMapLibrary.Map_Find` (`/Game/Player/PlayerCharacter.NumberOfKeys` _asplayer_character) (`self.KeyTypeEnum`)) 0)
        (`self.UpdateUIMessage` "Press \"E\" to open the door")
        (else
          (`self.UpdateUIMessage` "You will need a compatible Skull Key to open this door"))))))

(event `InputAction|Interact`
  (params (Key :type "Key Structure"))
  (bind _keytypeenum (`self.KeyTypeEnum`))
  (:`Pressed`
    (bind _asplayer_character (cast `/Game/Player/PlayerCharacter` (`GameplayStatics.GetPlayerCharacter` 0)))
    (bind _numberofkeys (`/Game/Player/PlayerCharacter.NumberOfKeys` _asplayer_character))
    (bind _value (`BlueprintMapLibrary.Map_Find` _numberofkeys _keytypeenum))
    (if (> _value 0)
      (bind _result (`/Engine/EditorBlueprintResources/StandardMacros.DecrementInt` _value)
        (:`  `
          (`BlueprintMapLibrary.Map_Add` _numberofkeys _keytypeenum _result)
          (`self.UpdateUIMessage` "")
          (bind _asmaze_game_mode (cast `/Game/GameMode/MazeGameMode` (`GameplayStatics.GetGameMode`)))
          (`/Game/UI/HUD.UpdateSkulls` (`/Game/GameMode/MazeGameMode.HUD` _asmaze_game_mode) "NewEnumerator0")
          (bind _returnvalue (`AddComponent|NODE_AddStaticMeshComponent-0`))
          (bind _asmaze_game_instance (cast `/Game/GameMode/MazeGameInstance` (`GameplayStatics.GetGameInstance`)))
          (bind _output_get (set `self.KeyMesh` _returnvalue))
          (`PrimitiveComponent.SetMaterial` _output_get 0 (`BlueprintMapLibrary.Map_Find` (`/Game/GameMode/MazeGameInstance.KeyTypes` _asmaze_game_instance) (`self.KeyTypeEnum`)))
          (`SceneComponent.K2_AttachToComponent` _output_get (`self.Keyhole`) "None" "SnapToTarget" "SnapToTarget" "SnapToTarget" true)
          (set `self.open` true)
          (`self.DisableInput` (`GameplayStatics.GetPlayerController` 0))
          (`GameplayStatics.PlaySoundAtLocation` "/Game/Sounds/DoorOpening_SFX.DoorOpening_SFX" (`SceneComponent.K2_GetComponentLocation` (`self.DoorMesh`)) (struct) 1.0 1.0 0.0 null null null)
          (bind (_direction _doorposition _keyposition) (`Timeline|DoorOpening` :!via `PlayFromStart`)
            (:`Update`
              (`SceneComponent.K2_SetRelativeLocation` (`self.KeyMesh`) (`KismetMathLibrary.MakeVector` 0.0 _keyposition) false false)
              (`SceneComponent.K2_SetRelativeLocation` (`self.DoorMesh`) (`KismetMathLibrary.MakeVector` 0.0 0.0 _doorposition) false false))
            (:`Finished`
              (`self.K2_DestroyActor`))))))))

(event `self.TriggerVolume.OnComponentEndOverlap`
  (params (OverlappedComponent :type "PrimitiveComponent Object Reference") (OtherActor :type "Actor Object Reference") (OtherComp :type "PrimitiveComponent Object Reference") (OtherBodyIndex :type Integer))
  (if (`self.open`)
    _
    (elif (== OtherActor (`GameplayStatics.GetPlayerCharacter` 0))
      (`self.DisableInput` (`GameplayStatics.GetPlayerController` 0))
      (`self.UpdateUIMessage` ""))))

(fn `UpdateUIMessage`
  (params (Message :type Text))
  (bind _asmaze_game_mode (cast `/Game/GameMode/MazeGameMode` (`GameplayStatics.GetGameMode`)))
  (bind _hud (`/Game/GameMode/MazeGameMode.HUD` _asmaze_game_mode))
  (set `/Game/UI/HUD.Message` Message _hud)
  (`/Game/UI/HUD.UpdateMessage` _hud))

(fn `UserConstructionScript`)