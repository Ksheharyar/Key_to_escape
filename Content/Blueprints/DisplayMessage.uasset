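; DisplayMessage is a trigger Blueprint that shows a configurable text message on the maze game's HUD while the player stands inside its Box.
; Box overlap events filter for the player character, passing the Message variable on entry and an empty string on exit.
; UpdateUIMessage casts the game mode to MazeGameMode, writes the text into its HUD's Message and calls UpdateMessage to refresh it.
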(event `self.Box.OnComponentBeginOverlap`
  (params (OverlappedComponent :type "PrimitiveComponent Object Reference") (OtherActor :type "Actor Object Reference") (OtherComp :type "PrimitiveComponent Object Reference") (OtherBodyIndex :type Integer) (bFromSweep :type Boolean) (SweepResult :type "HitResult Structure (by ref)"))
  (if (== OtherActor (`GameplayStatics.GetPlayerCharacter` 0))
    (`self.UpdateUIMessage` (`self.Message`))))

(event `self.Box.OnComponentEndOverlap`
  (params (OverlappedComponent :type "PrimitiveComponent Object Reference") (OtherActor :type "Actor Object Reference") (OtherComp :type "PrimitiveComponent Object Reference") (OtherBodyIndex :type Integer))
  (if (== OtherActor (`GameplayStatics.GetPlayerCharacter` 0))
    (`self.UpdateUIMessage` "")))

(fn `UpdateUIMessage`
  (params (Message :type Text))
  (bind _asmaze_game_mode (cast `/Game/GameMode/MazeGameMode` (`GameplayStatics.GetGameMode`)))
  (bind _hud (`/Game/GameMode/MazeGameMode.HUD` _asmaze_game_mode))
  (set `/Game/UI/HUD.Message` Message _hud)
  (`/Game/UI/HUD.UpdateMessage` _hud))

(fn `UserConstructionScript`)