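; BurstShooter is an actor that automatically fires Arrow actors in repeating bursts of three, starting at BeginPlay.
; Each shot spawns an Arrow at the ArrowSpawn component's transform and plays a sound at the mesh's location.
; A ShootCount counter drives a self-looping Delay chain, with a short gap between shots and a longer pause after each burst, without Tick or timers.
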(event `self.ReceiveBeginPlay`
  (bind _shootcount (`self.ShootCount`))
  (`|SpawnActorFromClass` "/Game/Blueprints/Arrow.Arrow_C" (`SceneComponent.K2_GetComponentToWorld` (`self.ArrowSpawn`)) "Undefined" "OverrideRootScale" null null :!label _label)
  (`GameplayStatics.PlaySoundAtLocation` "/Game/Sounds/Arrow_SFX.Arrow_SFX" (`SceneComponent.K2_GetComponentLocation` (`self.Mesh`)) (struct) 1.0 1.0 0.0 null null null)
  (if (== _shootcount 2)
    (set `self.ShootCount` 0)
    (`KismetSystemLibrary.Delay` 2.5)
    (goto _label)
    (else
      (`/Engine/EditorBlueprintResources/StandardMacros.IncrementInt` _shootcount
        (:`  `
          (`KismetSystemLibrary.Delay` 0.3)
          (goto _label))))))

(fn `UserConstructionScript`)