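; Shooter actor that fires arrows whenever the player character crosses its line of sight.
; Each tick, a sphere trace on the Camera channel runs forward from the ArrowSpawn component and calls ShootArrow when it hits the player.
; After a short delay, ShootArrow spawns an Arrow at that component and plays a sound, with a DoOnce and delayed reset acting as the cooldown.
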(event `ShootArrow`
  (`KismetSystemLibrary.Delay` 0.2)
  (`/Engine/EditorBlueprintResources/StandardMacros.DoOnce` false :!label _label
    (:`Completed`
      (`|SpawnActorFromClass` "/Game/Blueprints/Arrow.Arrow_C" (`SceneComponent.K2_GetComponentToWorld` (`self.ArrowSpawn`)) "Undefined" "OverrideRootScale" null null)
      (`GameplayStatics.PlaySoundAtLocation` "/Game/Sounds/Arrow_SFX.Arrow_SFX" (`SceneComponent.K2_GetComponentLocation` (`self.Mesh`)) (struct) 1.0 1.0 0.0 null null null)
      (`KismetSystemLibrary.Delay` 2.0)
      (goto _label :!via `Reset`))))

(event `self.ReceiveTick`
  (params (DeltaSeconds :type "Float (single-precision)"))
  (bind _arrowspawn (`self.ArrowSpawn`))
  (bind _returnvalue (`SceneComponent.K2_GetComponentLocation` _arrowspawn))
  (bind _returnvalue_2 (`KismetMathLibrary.GetForwardVector` (`SceneComponent.K2_GetComponentRotation` _arrowspawn)))
  (bind _outhit (`KismetSystemLibrary.SphereTraceSingle` (+ _returnvalue (* _returnvalue_2 50)) (+ _returnvalue (* _returnvalue_2 3000)) 30.0 "TraceTypeQuery2"))
  (if (== (`.HitActor` (`GameplayStatics.BreakHitResult` _outhit)) (`GameplayStatics.GetPlayerCharacter` 0))
    (`self.ShootArrow`)))

(fn `UserConstructionScript`)