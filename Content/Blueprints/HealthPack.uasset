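; Health pickup that heals the player character by one point on overlap if health is below 3, using negative ApplyDamage.
; An idle timeline rotates the mesh and pulses its scale along with the point light radius.
; On pickup, a Used flag stops the pulse while a Vanish timeline, offset by the current scale, drives mesh and light before destroying the actor.
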(event `self.ReceiveBeginPlay`
  (bind _output_get (set `self.LightRadius` (`LocalLightComponent.AttenuationRadius` (`self.PointLight`))))
  (bind (_direction _scale _rotation) (`Timeline|IdleAnimation` :!via `PlayFromStart`)
    (:`Update`
      (`SceneComponent.K2_SetRelativeRotation` (`self.Mesh`) (`KismetMathLibrary.MakeRotator` 0.0 0.0 _rotation) false false)
      (if (not (`self.Used`))
        (`SceneComponent.SetRelativeScale3D` (`self.Mesh`) (`KismetMathLibrary.Conv_DoubleToVector` _scale))
        (`LocalLightComponent.SetAttenuationRadius` (`self.PointLight`) (* _scale _output_get))))))

(event `self.Trigger.OnComponentBeginOverlap`
  (params (OverlappedComponent :type "PrimitiveComponent Object Reference") (OtherActor :type "Actor Object Reference") (OtherComp :type "PrimitiveComponent Object Reference") (OtherBodyIndex :type Integer) (bFromSweep :type Boolean) (SweepResult :type "HitResult Structure (by ref)"))
  (bind _returnvalue (`GameplayStatics.GetPlayerCharacter` 0))
  (bind _relativescale3d_x (`KismetMathLibrary.BreakVector` (`SceneComponent.RelativeScale3D` (`self.Mesh`))))
  (if (and (not (`self.Used`)) (== OtherActor _returnvalue))
    (bind _asplayer_character (cast `/Game/Player/PlayerCharacter` _returnvalue))
    (if (< (`/Game/Player/PlayerCharacter.Health` _asplayer_character) 3)
      (`GameplayStatics.ApplyDamage` _asplayer_character -1.0)
      (set `self.Used` true)
      (bind (_direction _vanish) (`Timeline|Vanish` :`NewTime` (- 0.5 (/ _relativescale3d_x 2.0)))
        (:`Update`
          (`SceneComponent.SetRelativeScale3D` (`self.Mesh`) (`KismetMathLibrary.Conv_DoubleToVector` _vanish))
          (`LocalLightComponent.SetAttenuationRadius` (`self.PointLight`) (* _vanish (`self.LightRadius`))))
        (:`Finished`
          (`self.K2_DestroyActor`))))))

(fn `UserConstructionScript`)